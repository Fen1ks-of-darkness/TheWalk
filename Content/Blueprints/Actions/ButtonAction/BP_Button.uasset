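; BP_Button is an interactable button that slides a target object open along X when pushed.
; Interact messages the player character to move to the MoveToTarget point, passing the button, a linked actor and Alex's push montage.
; After a fixed delay, a timeline subtracts its value from the target's current world X every update and sets that as relative location, so movement accumulates per frame.
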(event `/Game/Blueprints/Characters/Interfaces/BPI_Interact.Interact`
  (message `/Game/Blueprints/Characters/Interfaces/BPI_Interact.MoveTo` (`GameplayStatics.GetPlayerCharacter` 0) (`SceneComponent.K2_GetComponentLocation` (`self.MoveToTarget`)) self (`self.LinkedActor`) "/Game/Assets/Characters/Alex/Animations/Sequences/Montages/Actions/AM_Alex_PushButton.AM_Alex_PushButton")
  (`KismetSystemLibrary.Delay` 1.33)
  (bind (_direction _openingtoleft) (`Timeline|OpeningObjectToLeft` :!via `PlayFromStart`)
    (:`Update`
      (`self.K2_SetActorRelativeLocation` (`self.TargetObject`) (`KismetMathLibrary.MakeVector` (- (.x (`self.K2_GetActorLocation` (`self.TargetObject`))) (.x _openingtoleft)) (.y (`self.K2_GetActorLocation` (`self.TargetObject`))) (.z (`self.K2_GetActorLocation` (`self.TargetObject`)))) false false))))

(fn `UserConstructionScript`)