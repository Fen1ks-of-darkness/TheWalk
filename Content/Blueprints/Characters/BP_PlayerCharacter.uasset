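; Player character with walking, running with camera shake, jumping, a socketed flashlight and sphere-trace interaction through BPI_Interact.
; Tick box-traces for actors tagged Vault or Mantle at walking speed, then plays collision-free montages in flying mode.
; The B key attaches to ledges by capsule trace and timelines, reading ledge yaw from actor tags.
; Move input drives directional climbing montages through motion warping, and Jump climbs onto ledges tagged Up.
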(event `self.ReceiveBeginPlay`
  ; BeginPlay
  (bind _astwcharacter_movement_component (cast `TWCharacterMovementComponent` (`self.CharacterMovement`)))
  (set `self.CharacterMovementComp` _astwcharacter_movement_component)
  (set `self.ShouldTurnInPlace` true))

(event `self.ReceiveTick`
  (params (DeltaSeconds :type "Float (single-precision)"))
  (bind _charactermovementcomp (`self.CharacterMovementComp`))
  (bind _charactermovementcomp_2 (`self.CharacterMovementComp`))
  ; Event Tick / Turn In Place / Traversal System
  (if (<= (`KismetMathLibrary.VSize` (`MovementComponent.Velocity` (`self.CharacterMovementComp`))) 1.0)
    (set `self.ShouldTurnInPlace` true)
    (else
      (set `self.ShouldTurnInPlace` false)
      (if (<= (`KismetMathLibrary.VSize` (`MovementComponent.Velocity` (`self.CharacterMovementComp`))) 199.7)
        (bind _tracegothit (`self.TraversalTypeDetection`))
        (if _tracegothit
          (`|ExecutionSequence`
            (:`then_0`
              (if (`self.TraversalVault`)
                (`/Engine/EditorBlueprintResources/StandardMacros.DoOnce` false :!label _label
                  (:`Completed`
                    (`CharacterMovementComponent.SetMovementMode` _charactermovementcomp_2 "MOVE_Flying" 0)
                    (set `CharacterMovementComponent.MaxFlySpeed` 0.0 _charactermovementcomp_2)
                    (set `self.CanProcessInput` false)
                    (`PrimitiveComponent.SetCollisionEnabled` (`self.CapsuleComponent`) "NoCollision")
                    (`PrimitiveComponent.SetCollisionEnabled` (`self.Mesh`) "NoCollision")
                    (`|PlayMontage` (`self.Mesh`) "/Game/Assets/Characters/Alex/Animations/Sequences/Montages/Traversal/AS_Alex_Vault_Montage.AS_Alex_Vault_Montage" 1.3
                      (:`OnCompleted`
                        (`self.StopMontage`)
                        (set `self.TraversalVault` false)
                        (goto _label :!via `Reset`)))))))
            (:`then_1`
              (if (`self.TraversalMantle`)
                (`/Engine/EditorBlueprintResources/StandardMacros.DoOnce` false :!label _label_2
                  (:`Completed`
                    (`CharacterMovementComponent.SetMovementMode` _charactermovementcomp "MOVE_Flying" 0)
                    (set `CharacterMovementComponent.MaxFlySpeed` 0.0 _charactermovementcomp)
                    (set `self.CanProcessInput` false)
                    (`PrimitiveComponent.SetCollisionEnabled` (`self.CapsuleComponent`) "NoCollision")
                    (`PrimitiveComponent.SetCollisionEnabled` (`self.Mesh`) "NoCollision")
                    (`|PlayMontage` (`self.Mesh`) "/Game/Assets/Characters/Alex/Animations/Sequences/Montages/Traversal/AS_Alex_Mantle_Montage.AS_Alex_Mantle_Montage" 1.2
                      (:`OnCompleted`
                        (`self.StopMontage`)
                        (set `self.TraversalMantle` false)
                        (goto _label_2 :!via `Reset`)))))))))))))

(event `EnhancedInput|/Game/Data/Inputs/IA_Jump`
  (params (ActionValue :type Boolean) (ElapsedSeconds :type "Float (double-precision)") (TriggeredSeconds :type "Float (double-precision)") (InputAction :type "InputAction Object Reference" :default "/Game/Data/Inputs/IA_Jump.IA_Jump"))
  ; Jump / Ledge Up System
  (:`Triggered`
    (`/Engine/EditorBlueprintResources/StandardMacros.DoOnce` false :!label _label_3
      (:`Completed`
        (if (`NavMovementComponent.IsCrouching` (`self.CharacterMovementComp`))
          (goto _label_3 :!via `Reset`)
          (elif (`self.IsAlreadyClimbingLedge`)
            (`self.ClimbUpLedgeDetection`)
            (if (`self.ClimbUpHitDetected`)
              (set `self.LedgeNavTimelineFinished` false)
              (set `self.IsAlreadyClimbingLedge` false)
              (set `self.CanProcessInput` false)
              (`|PlayMontage` (`self.Mesh`) "/Game/Assets/Characters/Alex/Animations/Sequences/Montages/LedgeClimb/AS_Alex_LedgeClimbUpToTop_Montage.AS_Alex_LedgeClimbUpToTop_Montage" 1.0 0.56
                (:`OnCompleted`
                  (`self.StopMontage`)
                  (goto _label_3 :!via `Reset`))))
            (else
              (`self.Jump`)
              (`GameplayStatics.PlaySound2D` "/Game/Assets/Sounds/Characters/Alex/Jump/Alex_Jump_Cue.Alex_Jump_Cue" 1.0 1.0 0.0 null null)
              (`KismetSystemLibrary.Delay` 1.0)
              (goto _label_3 :!via `Reset`)))))))
  (:`Completed`
    (`self.StopJumping`)))

(event `EnhancedInput|/Game/Data/Inputs/IA_Move`
  (params (ActionValue :type "Vector2D Structure") (ElapsedSeconds :type "Float (double-precision)") (TriggeredSeconds :type "Float (double-precision)") (InputAction :type "InputAction Object Reference" :default "/Game/Data/Inputs/IA_Move.IA_Move"))
  (bind (_returnvalue_roll _returnvalue_pitch _returnvalue_yaw) (`KismetMathLibrary.BreakRotator` (`self.GetControlRotation`)))
  (bind (_targettransform_location _targettransform_rotation) (`KismetMathLibrary.BreakTransform` (`self.TargetTransform`)))
  (bind (_returnvalue_x _returnvalue_y) (`KismetMathLibrary.BreakVector2D` (`KismetMathLibrary.Normal2D` (`self.MovementInput`))))
  ; Character Movement / Ledge System
  (:`Triggered`
    (set `self.MovementInput` ActionValue)
    (`self.ActionValuesManagementMacro` :!label _label_4)
    (if (`self.IsAlreadyClimbingLedge`)
      (bind _didhitledge_ (`self.LedgeTraceDetection`))
      (if _didhitledge_
        (if (`self.IsAlreadyClimbingLedge`)
          (if (`self.LedgeNavTimelineFinished`)
            (if (or (!= (`self.ActionValueX`) 0.0) (!= (`self.ActionValueY`) 0.0))
              (set `self.SavedActionValueX` (`self.ActionValueX`))
              (set `self.SavedActionValueY` (`self.ActionValueY`))
              (if (`self.LedgeHitDetected`)
                (`self.ProccesLedgeTargetData`)
                (bind _foundvaliddirection (`self.DetermineLedgeAngle`))
                (if _foundvaliddirection
                  (bind _ledgeselectiondirection (`self.LedgeMontageSelectorByDirection`))
                  (if (`|EnumInequality` _ledgeselectiondirection "NewEnumerator8")
                    (set `self.LedgeNavTimelineFinished` false)
                    (`/Engine/EditorBlueprintResources/StandardMacros.DoOnce` false :!label _label_5
                      (:`Completed`
                        (`MotionWarpingComponent.AddOrUpdateWarpTarget` (`self.MotionWarping`) (make `MotionWarpingTarget` "LedgeWarp" (- _targettransform_location (0.0 0.0 95.0)) _targettransform_rotation (`self.CapsuleComponent`)))
                        (`|PlayMontage` (`self.Mesh`) (`self.LedgeMontageToPlay`) (`self.Playrate`) (`self.StartingPosition`)
                          (:`then`
                            (`KismetSystemLibrary.RetriggerableDelay` 1.2)
                            (set `self.CurrentLedgeAngle` (`self.TargetedLedgeAngle`))
                            (set `self.LedgeNavTimelineFinished` true)
                            (goto _label_5 :!via `Reset`))
                          (:`OnCompleted`
                            (`MovementComponent.StopMovementImmediately` (`self.CharacterMovementComp`)))))))))
              (else
                (set `self.SavedActionValueY` 1.0)
                (set `self.SavedActionValueX` 0.0))))))
      (else
        (`self.AddMovementInput` (`KismetMathLibrary.GetRightVector` (`KismetMathLibrary.MakeRotator` 0.0 0.0 _returnvalue_yaw)) _returnvalue_x)
        (`self.AddMovementInput` (`KismetMathLibrary.GetForwardVector` (`KismetMathLibrary.MakeRotator` 0.0 0.0 _returnvalue_yaw)) _returnvalue_y))))
  (:`Canceled`
    (set `self.MovementInput` ActionValue :!label _label_6)
    (goto _label_4 :!via `Canceled / completed`))
  (:`Completed`
    (goto _label_6)))

(event `EnhancedInput|/Game/Data/Inputs/IA_Run`
  (params (ActionValue :type Boolean) (ElapsedSeconds :type "Float (double-precision)") (TriggeredSeconds :type "Float (double-precision)") (InputAction :type "InputAction Object Reference" :default "/Game/Data/Inputs/IA_Run.IA_Run"))
  (bind _camerashakesourcecomponent (`self.CameraShakeSourceComponent`))
  (bind _camerashakesourcecomponent_2 (`self.CameraShakeSourceComponent`))
  (bind _charactermovementcomp (`self.CharacterMovementComp`))
  ; When Running start Camera Shake + turn face the direction of travel
  (:`Triggered`
    (if (`self.CanProcessInput`)
      (if (and (>= (`KismetMathLibrary.VSize` (`MovementComponent.Velocity` _charactermovementcomp)) 1.0) (not (`NavMovementComponent.IsCrouching` _charactermovementcomp)))
        (set `self.bImmediatelyStopCameraShake?` false)
        (set `TWCameraShakeSourceComponent.Threshold` 0.7 _camerashakesourcecomponent)
        (set `TWCharacterMovementComponent.MovementType` "Running" (`self.CharacterMovementComp`))
        (`CameraShakeSourceComponent.StartCameraShake` :`self` _camerashakesourcecomponent :`InCameraShake` "/Game/Blueprints/Characters/CameraShake/BP_CameraShake.BP_CameraShake_C"))))
  (:`Completed`
    (set `TWCharacterMovementComponent.MovementType` "Walking" (`self.CharacterMovementComp`))
    (bind (_direction _shake) (`Timeline|SmoothCameraShake` :!via `PlayFromStart` :!label _label_7)
      (:`Update`
        (bind _output_get (set `TWCameraShakeSourceComponent.Threshold` _shake _camerashakesourcecomponent_2))
        (if (== _output_get 1.0)
          (`CameraShakeSourceComponent.StopAllCameraShakes` _camerashakesourcecomponent_2 (`self.bImmediatelyStopCameraShake?`))
          (`KismetSystemLibrary.Delay` 0.25)
          (set `self.bImmediatelyStopCameraShake?` true)
          (goto _label_7 :!via `Stop`))))))

(event `EnhancedInput|/Game/Data/Inputs/IA_FlashlightOnOff`
  (params (ActionValue :type Boolean) (ElapsedSeconds :type "Float (double-precision)") (TriggeredSeconds :type "Float (double-precision)") (InputAction :type "InputAction Object Reference" :default "/Game/Data/Inputs/IA_FlashlightOnOff.IA_FlashlightOnOff"))
  (bind _spotlight (`self.SpotLight`))
  (bind _returnvalue (`SceneComponent.K2_GetComponentLocation` (`self.Flashlight`)))
  ; Turn On \ Off = Flashlight
  (:`Started`
    (`/Engine/EditorBlueprintResources/StandardMacros.FlipFlop`
      (:`A`
        (`SceneComponent.SetVisibility` _spotlight true false)
        (`GameplayStatics.PlaySoundAtLocation` "/Game/Assets/Sounds/Flashlight/Flashlight_On_Cue.Flashlight_On_Cue" _returnvalue (struct) 1.0 1.0 0.0 null null null null))
      (:`B`
        (`SceneComponent.SetVisibility` _spotlight false false)
        (`GameplayStatics.PlaySoundAtLocation` "/Game/Assets/Sounds/Flashlight/Flashlight_Off_Cue.Flashlight_Off_Cue" _returnvalue (struct) 1.0 1.0 0.0 null null null null)))))

(event `EnhancedInput|/Game/Data/Inputs/IA_Interaction`
  (params (ActionValue :type Boolean) (ElapsedSeconds :type "Float (double-precision)") (TriggeredSeconds :type "Float (double-precision)") (InputAction :type "InputAction Object Reference" :default "/Game/Data/Inputs/IA_Interaction.IA_Interaction"))
  ; Push Button Interact
  (:`Triggered`
    (if (not (`self.Interacting`))
      (`self.InteractTrace`))))

(event `Key|B`
  (params (Key :type "Key Structure"))
  (bind _returnvalue (`self.K2_GetActorLocation`))
  (bind _charactermovementcomp (`self.CharacterMovementComp`))
  (bind _charactermovementcomp_2 (`self.CharacterMovementComp`))
  (bind _returnvalue_2 (`KismetSystemLibrary.MakeLiteralDouble` (`KismetStringLibrary.Conv_StringToDouble` (`KismetStringLibrary.Conv_NameToString` (`|GetArrayItem` (`Actor.Tags` (`.HitActor` (`GameplayStatics.BreakHitResult` (`self.HangTrace`)))))))))
  (:`Pressed`
    (if (`self.CanAttachToLedge`)
      (if (`self.IsAlreadyClimbingLedge`)
        (`TimelineComponent.Stop` (`self.LocationTimelineCharacter`))
        (`TimelineComponent.Stop` (`self.RotationTimelineCharacter`))
        (`self.StopMontage`)
        (elif (`self.CanProcessInput`)
          (bind (_outhit _returnvalue_3) (`KismetSystemLibrary.CapsuleTraceSingleForObjects` :`Start` (+ (* (`self.GetActorForwardVector`) 16.0) _returnvalue (0.0 0.0 18.0)) :`End` (+ _returnvalue (0.0 0.0 0.2) (* (`self.GetActorForwardVector`) 10.5)) :`Radius` 37.0 :`HalfHeight` 68.0 :`ObjectTypes` (`|MakeArray` "ObjectTypeQuery8" :!type "EObjectTypeQuery Enum") :`DrawDebugType` "ForDuration" :`DrawTime` 3.0))
          (set `self.HangTrace` _outhit)
          (if _returnvalue_3
            (set `self.CanProcessInput` false)
            (set `self.CanAttachToLedge` false)
            (`CharacterMovementComponent.SetMovementMode` _charactermovementcomp_2 "MOVE_Flying" 0)
            (`MovementComponent.StopMovementImmediately` _charactermovementcomp_2)
            (set `CharacterMovementComponent.MaxFlySpeed` 0.0 _charactermovementcomp_2)
            (`PrimitiveComponent.SetCollisionEnabled` (`self.CapsuleComponent`) "NoCollision")
            (`PrimitiveComponent.SetCollisionEnabled` (`self.Mesh`) "NoCollision")
            (set `CharacterMovementComponent.bOrientRotationToMovement` false _charactermovementcomp)
            (set `CharacterMovementComponent.bUseControllerDesiredRotation` false _charactermovementcomp)
            (set `self.IsAlreadyClimbingLedge` true)
            (set `self.DidHitTraceFirstAttachment` true)
            (if (`self.DidHitTraceFirstAttachment`)
              (set `self.CurrentLedgeAngle` _returnvalue_2)
              (`self.K2_SetActorRotation` (`KismetMathLibrary.MakeRotator` 0.0 0.0 _returnvalue_2))
              (set `self.CurrentLocation` (`self.K2_GetActorLocation`))
              (set `self.TargetLocation` (+ (`.ImpactPoint` (`GameplayStatics.BreakHitResult` (`self.HangTrace`))) (* (`self.GetActorForwardVector`) (* (`KismetMathLibrary.Abs` (`self.InitLedgeForwardOffset`)) -1.0)) (* (`self.GetActorUpVector`) (`self.InitLedgeVercticalOffset`))))
              (set `self.LocationTimelineFinished` false)
              (set `self.RotationTimelineFinished` false)
              (`TimelineComponent.PlayFromStart` (`self.LocationTimelineCharacter`))
              (`TimelineComponent.PlayFromStart` (`self.RotationTimelineCharacter`)))
            (else
              (set `self.DidHitTraceFirstAttachment` false))))))))

(fn `ClimbUpLedgeDetection`
  (returns (`ClimbUpHitDetected?` :type Boolean))
  (bind _returnvalue (+ (`self.K2_GetActorLocation`) (+ (`self.GetActorUpVector`) (0.0 0.0 25.0)) (* (`self.GetActorForwardVector`) 55.0) (0.0 0.0 25.0)))
  (bind (_outhit _returnvalue_2) (`KismetSystemLibrary.BoxTraceSingleForObjects` :`Start` _returnvalue :`End` _returnvalue :`HalfSize` (25.0 25.0 15.0) :`ObjectTypes` (`|MakeArray` "ObjectTypeQuery8" :!type "EObjectTypeQuery Enum") :`DrawDebugType` "ForDuration" :`TraceColor` (struct :`R` 1.0 :`G` 0.970606 :`B` 0.939261 :`A` 1.0)))
  (if _returnvalue_2
    (if (`self.ActorHasTag` (`.HitActor` (`GameplayStatics.BreakHitResult` _outhit)) "Up")
      (set `self.ClimbUpHitDetected` true)
      (else
        (set `self.ClimbUpHitDetected` false)))
    (return (`self.ClimbUpHitDetected`))))

(fn `DetermineLedgeAngle`
  (returns (FoundValidDirection :type Boolean))
  (if (`self.LedgeInputParameter` -0.3 0.3 0.8 1.0)
    (set `self.LedgeSelectionDirection` "NewEnumerator0")
    (return true)
    (elif (`self.LedgeInputParameter` -0.3 0.3 -1.0 -0.8)
      (set `self.LedgeSelectionDirection` "NewEnumerator4")
      (return true)
      (elif (`self.LedgeInputParameter` 0.3 1.0 0.3 1.0)
        (set `self.LedgeSelectionDirection` "NewEnumerator1")
        (return true)
        (elif (`self.LedgeInputParameter` 0.8 1.0 -1.0 0.7)
          (set `self.LedgeSelectionDirection` "NewEnumerator2")
          (return true)
          (elif (`self.LedgeInputParameter` 0.3 1.0 -1.0 -0.3)
            (set `self.LedgeSelectionDirection` "NewEnumerator3")
            (return true)
            (elif (`self.LedgeInputParameter` -1.0 -0.3 -1.0 -0.3)
              (set `self.LedgeSelectionDirection` "NewEnumerator5")
              (return true)
              (elif (`self.LedgeInputParameter` -1.0 -0.3 -0.3 0.7)
                (set `self.LedgeSelectionDirection` "NewEnumerator6")
                (return true)
                (elif (`self.LedgeInputParameter` -1.0 -0.3 0.3 1.0)
                  (set `self.LedgeSelectionDirection` "NewEnumerator7")
                  (return true)
                  (else
                    (set `self.LedgeSelectionDirection` "NewEnumerator8")
                    (return false)))))))))))

(fn `InteractTrace`
  (bind _returnvalue (`self.K2_GetActorLocation`))
  (bind (_outhit _returnvalue_2) (`KismetSystemLibrary.SphereTraceSingleForObjects` _returnvalue (+ _returnvalue (* (`self.GetActorForwardVector`) 125.0)) 30.0 (`|MakeArray` "ObjectTypeQuery7" :!type "EObjectTypeQuery Enum")))
  (if _returnvalue_2
    (bind (_bblockinghit _binitialoverlap _time _distance _location _impactpoint _normal _impactnormal _physmat _hitactor) (`GameplayStatics.BreakHitResult` _outhit))
    (`/Engine/EditorBlueprintResources/StandardMacros.IsValid` _hitactor
      (:`Is Valid`
        (if (`KismetSystemLibrary.DoesImplementInterface` _hitactor "/Game/Blueprints/Characters/Interfaces/BPI_Interact.BPI_Interact_C")
          (message `/Game/Blueprints/Characters/Interfaces/BPI_Interact.Interact` _hitactor)
          (set `self.Interacting` true))))))

(fn `LedgeMontageSelectorByDirection`
  (returns (LedgeSelectionDirection :type "/Game/Data/MontageSelectionEnum Enum"))
  (set `self.LedgeMontageToPlay` null)
  (`|ExecutionSequence`
    (:`then_0`
      (if true
        (set `self.LedgeMontageToPlay` (select `/Game/Data/MontageSelectionEnum` (`self.LedgeSelectionDirection`) :`NewEnumerator0` "/Game/Assets/Characters/Alex/Animations/Sequences/Montages/LedgeClimb/AS_Alex_LedgeClimbingUp_Montage.AS_Alex_LedgeClimbingUp_Montage" :`NewEnumerator2` "/Game/Assets/Characters/Alex/Animations/Sequences/Montages/LedgeClimb/AS_Alex_LedgeClimbingRight_Montage.AS_Alex_LedgeClimbingRight_Montage" :`NewEnumerator4` "/Game/Assets/Characters/Alex/Animations/Sequences/Montages/LedgeClimb/AS_Alex_LedgeClimbingDown_Montage.AS_Alex_LedgeClimbingDown_Montage" :`NewEnumerator6` "/Game/Assets/Characters/Alex/Animations/Sequences/Montages/LedgeClimb/AS_Alex_LedgeClimbingLeft_Montage.AS_Alex_LedgeClimbingLeft_Montage" :!type "AnimMontage Object Reference"))
        (`self.SetLedgeParamsFromAngle` false 0.0 0.0 0.23)
        (else
          (set `self.LedgeSelectionDirection` "NewEnumerator8"))))
    (:`then_1`
      (return (`self.LedgeSelectionDirection`)))))

(fn `LedgeTraceDetection`
  (returns (`DidHitLedge?` :type Boolean))
  (bind _inputy (`self.InputY`))
  (bind _returnvalue (+ (`self.K2_GetActorLocation`) (* (`self.GetActorUpVector`) _inputy (`KismetMathLibrary.SelectFloat` 65.0 65.0 (`KismetMathLibrary.InRange_FloatFloat` _inputy))) (* (`self.GetActorRightVector`) (`self.InputX`) 50.0) (* (`self.GetActorForwardVector`) 25.0) (0.0 0.0 25.0)))
  (bind (_outhit _returnvalue_2) (`KismetSystemLibrary.CapsuleTraceSingleForObjects` :`Start` _returnvalue :`End` (+ _returnvalue (* (`self.GetActorUpVector`) (`self.InputY`) 120.0) (* (`self.GetActorRightVector`) (`self.InputX`) 120.0)) :`Radius` 30.0 :`HalfHeight` 25.0 :`ObjectTypes` (`|MakeArray` "ObjectTypeQuery8" :!type "EObjectTypeQuery Enum") :`DrawDebugType` "ForOneFrame" :`TraceColor` (struct :`R` 0.968478 :`G` 1.0 :`B` 0.957051 :`A` 1.0)))
  (if _returnvalue_2
    (set `self.LedgeHitDetected` true)
    (else
      (set `self.LedgeHitDetected` false)))
  (set `self.DynamicLedgeAttach` _outhit)
  (return (`self.LedgeHitDetected`)))

(fn `ProccesLedgeTargetData`
  (bind (_returnvalue_roll _returnvalue_pitch _returnvalue_yaw) (`KismetMathLibrary.BreakRotator` (`KismetMathLibrary.NormalizedDeltaRotator` (`KismetMathLibrary.MakeRotator` 0.0 0.0 (`self.CurrentLedgeAngle`)) (`KismetMathLibrary.MakeRotator` 0.0 0.0 (`self.TargetedLedgeAngle`)))))
  (bind (_returnvalue_x _returnvalue_y _returnvalue_z) (`KismetMathLibrary.BreakVector` (+ (`SceneComponent.K2_GetComponentLocation` (`self.Mesh`)) (`KismetMathLibrary.MakeVector` 0.0 0.0 110.0) (* (`self.GetActorForwardVector`) 35.0))))
  (bind (_returnvalue_x_2 _returnvalue_y_2 _returnvalue_z_2) (`KismetMathLibrary.BreakVector` (`KismetMathLibrary.GetForwardVector` (`KismetMathLibrary.FindRelativeLookAtRotation` (`KismetMathLibrary.MakeTransform` (`self.CharacterStartCenter`) (`self.K2_GetActorRotation`)) (`self.LedgeTargetEnd`)))))
  (set `self.CharacterStartCenter` (`KismetMathLibrary.MakeVector` _returnvalue_x _returnvalue_y _returnvalue_z))
  (set `self.LedgeTargetEnd` (`.ImpactPoint` (`GameplayStatics.BreakHitResult` (`self.DynamicLedgeAttach`))))
  (set `self.ReachDistance` (`KismetMathLibrary.Vector_Distance` (`self.CharacterStartCenter`) (`self.LedgeTargetEnd`)))
  (bind _output_get (set `self.TargetedLedgeAngle` (`KismetStringLibrary.Conv_StringToDouble` (`KismetStringLibrary.Conv_NameToString` (`|GetArrayItem` (`Actor.Tags` (`.HitActor` (`GameplayStatics.BreakHitResult` (`self.DynamicLedgeAttach`)))))))))
  (set `self.InitLedgeForwardOffset` 25.0)
  (set `self.TargetTransform` (`KismetMathLibrary.MakeTransform` (+ (* (`self.GetActorForwardVector`) (* (`self.InitLedgeForwardOffset`) -1.0)) (`self.LedgeTargetEnd`) (0.0 0.0 -47.0)) (`KismetMathLibrary.MakeRotator` 0.0 0.0 _output_get)))
  (set `self.SavedRotationX` (`KismetMathLibrary.MakeVector` _returnvalue_y_2 _returnvalue_z_2))
  (set `self.DeltaTargetAngle` _returnvalue_yaw)
  (return))

(fn `SetLedgeParamsFromAngle`
  (params (`UseSavedActorTransform?` :type Boolean) (AddPlayrate :type "Float (double-precision)") (StartingPosition :type "Float (double-precision)") (DelayUntilCorrection :type "Float (double-precision)"))
  (set `self.DelayUntilCorrection` DelayUntilCorrection)
  (set `self.UseSavedActorTransform?` (`self.UseSavedActorTransform?`))
  (set `self.Playrate` (+ AddPlayrate 1.0))
  (set `self.StartingPosition` StartingPosition))

(fn `StopMontage`
  (`AnimInstance.Montage_Stop` (`SkeletalMeshComponent.GetAnimInstance` (`self.Mesh`)) 0.25 null)
  (`CharacterMovementComponent.SetMovementMode` (`self.CharacterMovementComp`) "MOVE_Walking" 0)
  (`PrimitiveComponent.SetCollisionEnabled` (`self.CapsuleComponent`) "QueryAndPhysics")
  (`PrimitiveComponent.SetCollisionEnabled` (`self.Mesh`) "QueryAndPhysics")
  (set `self.LedgeNavTimelineFinished` true)
  (set `self.CanProcessInput` true)
  (set `self.IsAlreadyClimbingLedge` false)
  (set `self.CanAttachToLedge` true)
  (set `CharacterMovementComponent.bUseControllerDesiredRotation` true (`self.CharacterMovementComp`)))

(fn `TraversalTypeDetection`
  (returns (TraceGotHit :type Boolean))
  (bind _returnvalue (+ (`self.K2_GetActorLocation`) (+ (`self.GetActorUpVector`) (0.0 0.0 -15.0)) (* (`self.GetActorForwardVector`) 30.0) (0.0 0.0 25.0)))
  (bind (_outhit _returnvalue_2) (`KismetSystemLibrary.BoxTraceSingleForObjects` :`Start` _returnvalue :`End` _returnvalue :`HalfSize` (15.0 15.0 25.0) :`Orientation` (`self.K2_GetActorRotation`) :`ObjectTypes` (`|MakeArray` "ObjectTypeQuery9" :!type "EObjectTypeQuery Enum") :`DrawDebugType` "ForOneFrame" :`TraceColor` (struct :`R` 1.0 :`G` 0.970606 :`B` 0.939261 :`A` 1.0)))
  (if _returnvalue_2
    (bind (_bblockinghit _binitialoverlap _time _distance _location _impactpoint _normal _impactnormal _physmat _hitactor) (`GameplayStatics.BreakHitResult` _outhit))
    (set `self.TraversalVault` (`self.ActorHasTag` _hitactor "Vault"))
    (set `self.TraversalMantle` (`self.ActorHasTag` _hitactor "Mantle"))
    (return _returnvalue_2)))

(fn `UserConstructionScript`
  (set `self.ShouldTurnInPlace` true)
  (`SceneComponent.K2_AttachToComponent` (`self.Flashlight`) (`self.Mesh`) "Skt_Flashlight" "KeepRelative" "KeepRelative" "KeepRelative" true))