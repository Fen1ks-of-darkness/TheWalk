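; BP_Light is a light Blueprint that either flickers or holds a steady brightness, switched by ShouldBlink.
; When blinking, Tick re-sets a looping timer on Flickering every frame and also calls it after a BlinkRate delay.
; Flickering gives the FlickeringLight component a random intensity within a hardcoded range.
; Otherwise Tick applies LightIntensityIfNotBlink each frame, without clearing any timer already set.
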(event `self.ReceiveTick`
  (params (DeltaSeconds :type "Float (single-precision)"))
  (if (`self.bShouldBlink`)
    (`KismetSystemLibrary.K2_SetTimerDelegate` (delegate `Flickering`) 0.1 true)
    (`KismetSystemLibrary.Delay` (`self.BlinkRate`))
    (`self.Flickering`)
    (else
      (`LightComponent.SetIntensity` (`self.FlickeringLight`) (`self.LightIntensityIfNotBlink`)))))

(event `Flickering`
  (bind _output_get (set `self.New Intensity` 150.0))
  (`LightComponent.SetIntensity` (`self.FlickeringLight`) (`KismetMathLibrary.RandomFloatInRange` _output_get 1000.0)))

(fn `UserConstructionScript`)